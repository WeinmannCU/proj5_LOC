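; Spawner actor that keeps a BP_cheese available at its location.
; On BeginPlay, a looping timer runs CheckForBread every five seconds.
; The check looks for BP_cheese actors overlapping its Spawn component and, if none are present, spawns a new one at the spawner's transform.
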(event Custom|CheeseSpawn
  (Game|SpawnActorfromClass "/Game/GLBs/Cheese_Cut/StaticMeshes/BP_cheese.BP_cheese_C" (Transformation|GetActorTransform) "Undefined" "MultiplyWithRoot" 0 0))

(event Custom|CheckForBread
  (if (== (Utilities|Array|Length (Collision|GetOverlappingActors (Variables|Default|Getspawn) "/Game/GLBs/Cheese_Cut/StaticMeshes/BP_cheese.BP_cheese_C" :!class /Script/Engine.PrimitiveComponent)) 0)
    (CallFunction|CheeseSpawn)))

(event EventBeginPlay
  (Utilities|Time|SetTimerbyEvent (delegate Custom|CheckForBread) 5.0 true))

(event Collision|EventActorBeginOverlap
  (params (OtherActor :type Actor%20Object%20Reference)))

(event EventTick
  (params (DeltaSeconds :type Float%20%28single-precision%29)))

(fn ConstructionScript)