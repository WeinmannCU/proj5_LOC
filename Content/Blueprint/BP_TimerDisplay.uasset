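; BP_TimerDisplay shows a cook timer's progress through a widget component.
; On BeginPlay it casts the component's widget to WBP_MenuWidget and caches the reference.
; Every Tick it reads progress from the referenced BPCookTimer and pushes it to the widget's UpdateProgress.
; SwapColor sets the active index of the widget's WidgetSwitcher to switch the displayed variant.
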(event EventBeginPlay
  (bind _aswbp_menu_widget (Utilities|Casting|CastToWBP_MenuWidget (UserInterface|GetUserWidgetObject (Variables|Default|GetWidget))))
  (Variables|Default|SetMenuWidgetRef _aswbp_menu_widget))

(event EventTick
  (params (DeltaSeconds :type Float%20%28single-precision%29))
  (bind _progress (Default|GetTimerProgress (Variables|Default|GetBP_CookTimer)))
  (Default|UpdateProgress (Variables|Default|GetMenuWidgetRef) _progress))

(fn ConstructionScript)

(fn SwapColor
  (params (indexNum :type Integer))
  (Variables|/Script/UMG.WidgetSwitcher|SetActiveWidgetIndex (Variables|/Game/Blueprint/WBP_MenuWidget.WBP_MenuWidget_C|GetWidgetSwitcher (Variables|Default|GetMenuWidgetRef)) indexNum))