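; Knife spawner actor that keeps a Bp_knife available within its Spawn box volume.
; A looping timer started on BeginPlay periodically checks the box for overlapping knives and, if none is found, spawns one at a hard-coded world transform.
; Every Tick, it scans all Bp_knife actors in the level and destroys any whose location lies outside the box.
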(event Custom|KnifeSpawn
  (Game|SpawnActorfromClass "/Game/GLBs/Butter_knife/StaticMeshes/bp_knife.bp_knife_C" (Math|Transform|MakeTransform "311.000000,-150.000000,87.000000" "0.000000,180.000000,0.000000" "0.152500,0.152500,0.152500") "Undefined" "MultiplyWithRoot" 0 0))

(event Custom|CheckForKnife
  (if (== (Utilities|Array|Length (Collision|GetOverlappingActors (Variables|Default|Getspawn) "/Game/GLBs/Butter_knife/StaticMeshes/bp_knife.bp_knife_C" :!class /Script/Engine.PrimitiveComponent)) 0)
    (CallFunction|KnifeSpawn)))

(event EventBeginPlay
  (Utilities|Time|SetTimerbyEvent (delegate Custom|CheckForKnife) 5.0 true))

(event Collision|EventActorBeginOverlap
  (params (OtherActor :type Actor%20Object%20Reference)))

(event EventTick
  (params (DeltaSeconds :type Float%20%28single-precision%29))
  (bind _spawn (Variables|Default|Getspawn))
  (bind _outactors (Actor|GetAllActorsOfClass "/Game/GLBs/Butter_knife/StaticMeshes/bp_knife.bp_knife_C"))
  (for _array_element _outactors
    (if (not (Math|Geometry|IsPointinBox (Transformation|GetActorLocation _array_element) (Transformation|GetWorldLocation _spawn) (Components|Box|GetScaledBoxExtent _spawn)))
      (Actor|DestroyActor _array_element))))

(fn ConstructionScript)