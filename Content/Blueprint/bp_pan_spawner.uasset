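; Pan spawner actor that keeps a Pan present in its Spawn box and removes Pans found outside it.
; A looping timer from BeginPlay periodically checks the box's overlaps and spawns a Pan at a hardcoded world transform when none are inside.
; Every Tick, it scans all Pan actors in the level and destroys any whose location falls outside the box.
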(event Custom|CheckForPan
  (if (== (Utilities|Array|Length (Collision|GetOverlappingActors (Variables|Default|Getspawn) "/Game/FinalAssetBlueprints/Pan.Pan_C" :!class /Script/Engine.PrimitiveComponent)) 0)
    (Game|SpawnActorfromClass "/Game/FinalAssetBlueprints/Pan.Pan_C" (Math|Transform|MakeTransform "200.000000,50.000000,96.000000") "Undefined" "MultiplyWithRoot" 0 0)))

(event EventBeginPlay
  (Utilities|Time|SetTimerbyEvent (delegate Custom|CheckForPan) 5.0 true))

(event Collision|EventActorBeginOverlap
  (params (OtherActor :type Actor%20Object%20Reference)))

(event EventTick
  (params (DeltaSeconds :type Float%20%28single-precision%29))
  (bind _spawn (Variables|Default|Getspawn))
  (bind _outactors (Actor|GetAllActorsOfClass "/Game/FinalAssetBlueprints/Pan.Pan_C"))
  (for _array_element _outactors
    (if (not (Math|Geometry|IsPointinBox (Transformation|GetActorLocation _array_element) (Transformation|GetWorldLocation _spawn) (Components|Box|GetScaledBoxExtent _spawn)))
      (Actor|DestroyActor _array_element))))

(fn ConstructionScript)