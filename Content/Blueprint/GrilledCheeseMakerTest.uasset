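; Test actor for a grilled cheese maker that swaps a bread actor for a knife when play begins.
; On BeginPlay it spawns a Bp_knife at Bread1's location, then destroys Bread1.
; Unconnected nodes compute the average position of Bread1, Bread2 and Cheese as a transform, but nothing uses the result.
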(event EventBeginPlay
  (Game|SpawnActorfromClass "/Game/GLBs/Butter_knife/StaticMeshes/bp_knife.bp_knife_C" (Math|Conversions|ToTransform(Vector) (Transformation|GetActorLocation (Variables|Default|Getbread1))) "Undefined" "MultiplyWithRoot" 0 0)
  (Actor|DestroyActor (Variables|Default|Getbread1)))

(fn ConstructionScript)