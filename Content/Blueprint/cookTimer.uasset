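; cookTimer is a cooking timer that runs while all required actors overlap the Stove.
; Stove overlaps track required actors in ActorsInside, starting the timer when the count matches, while any end overlap resets it.
; A looping timer event, presumably UpdateTimer, accumulates ElapsedTime until TimerDuration, and GetTimerProgress returns the ratio.
; Finishing only prints and resets: TimerCompleted is never set true, and the looping timer is never cleared.
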(event Custom|OnActorBeginOverlap_Event_0
  (params (OverlappedActor :type Actor%20Object%20Reference) (OtherActor :type Actor%20Object%20Reference))
  (if (Utilities|Array|ContainsItem (Variables|Default|GetRequiredActors) OtherActor)
    (Utilities|Array|AddUnique (Variables|Default|GetActorsInside) OtherActor)
    (if (== (Utilities|Array|Length (Variables|Default|GetActorsInside)) (Utilities|Array|Length (Variables|Default|GetRequiredActors)))
      (Development|PrintString "Timer started!")
      (CallFunction|StartTimer)
      (else
        (Development|PrintString "Added Actor to Array")))))

(event Custom|OnActorEndOverlap_Event
  (params (OverlappedActor :type Actor%20Object%20Reference) (OtherActor :type Actor%20Object%20Reference))
  (Utilities|Array|RemoveItem (Variables|Default|GetActorsInside) OtherActor)
  (Development|PrintString "removed actor")
  (CallFunction|StopTimer))

(event EventBeginPlay
  (EventDispatchers|AssignOnActorBeginOverlap (Variables|Default|Getstove) (delegate Custom|OnActorBeginOverlap_Event_0))
  (EventDispatchers|AssignOnActorEndOverlap (Variables|Default|Getstove) (delegate Custom|OnActorEndOverlap_Event)))

(fn StartTimer
  (Variables|Default|SetElapsedTime 0.0)
  (Variables|Default|SetIsRunning true)
  (Variables|Default|SetTimerCompleted false)
  (Utilities|Time|SetTimerbyEvent (EventDispatchers|CreateEvent :!event UpdateTimer) 0.05 true))

(fn UpdateTimer
  (if (Variables|Default|GetIsRunning)
    (bind _output_get (Variables|Default|SetElapsedTime (+ (Variables|Default|GetElapsedTime) 0.05)))
    (if (>= _output_get (Variables|Default|GetTimerDuration))
      (Variables|Default|SetIsRunning false)
      (Variables|Default|SetTimerCompleted false)
      (Variables|Default|SetElapsedTime 0.0)
      (Development|PrintString "Timer finished!"))))

(fn StopTimer
  (Variables|Default|SetIsRunning false)
  (Variables|Default|SetTimerCompleted false)
  (Variables|Default|SetElapsedTime 0.0)
  (Development|PrintString "Reset Timer"))

(fn GetTimerProgress
  (return (/ (Variables|Default|GetElapsedTime) (Variables|Default|GetTimerDuration))))