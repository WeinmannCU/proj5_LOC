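; Cooking timer actor that turns ingredients on a stove into a grilled cheese, then a burnt one if left.
; Stove overlaps track required actors, starting the timer when all are present and resetting it when one leaves.
; Looping 0.05s timers advance a shared elapsed time through cook and burn phases, recoloring BP_TimerDisplay.
; SwapMesh spawns the resulting food near the first ingredient and destroys all but that ingredient.
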(event Custom|OnActorBeginOverlap_Event_0
  (params (OverlappedActor :type Actor%20Object%20Reference) (OtherActor :type Actor%20Object%20Reference))
  (if (Utilities|Array|ContainsItem (Variables|Default|GetRequiredActors) OtherActor)
    (Utilities|Array|AddUnique (Variables|Default|GetActorsInside) OtherActor)
    (if (== (Utilities|Array|Length (Variables|Default|GetActorsInside)) (Utilities|Array|Length (Variables|Default|GetRequiredActors)))
      (Development|PrintString "Timer started!")
      (CallFunction|StartTimer)
      (Variables|Default|SetisCooked true)
      (else
        (Development|PrintString "Added Actor to Array")))))

(event Custom|OnActorEndOverlap_Event
  (params (OverlappedActor :type Actor%20Object%20Reference) (OtherActor :type Actor%20Object%20Reference))
  (Utilities|Array|RemoveItem (Variables|Default|GetActorsInside) OtherActor)
  (Development|PrintString "removed actor")
  (CallFunction|StopTimer)
  (Variables|Default|SetisCooked false))

(event EventBeginPlay
  (EventDispatchers|AssignOnActorBeginOverlap (Variables|Default|Getstove) (delegate Custom|OnActorBeginOverlap_Event_0))
  (EventDispatchers|AssignOnActorEndOverlap (Variables|Default|Getstove) (delegate Custom|OnActorEndOverlap_Event)))

(fn ConstructionScript)

(fn StartTimer
  (Variables|Default|SetElapsedTime 0.0)
  (Variables|Default|SetIsRunning true)
  (Variables|Default|SetTimerCompleted false)
  (bind _returnvalue (Actor|GetActorOfClass "/Game/Blueprint/BP_TimerDisplay.BP_TimerDisplay_C"))
  (Default|SwapColor _returnvalue)
  (if (Variables|Default|GetisCooked)
    (Variables|Default|SetburntIsRunning true)
    (bind _returnvalue_2 (Actor|GetActorOfClass "/Game/Blueprint/BP_TimerDisplay.BP_TimerDisplay_C"))
    (Default|SwapColor _returnvalue_2 1)
    (Utilities|Time|SetTimerbyEvent (EventDispatchers|CreateEvent :!event BurnUpdateTimer) 0.05 true)
    (else
      (Utilities|Time|SetTimerbyEvent (EventDispatchers|CreateEvent :!event UpdateTimer) 0.05 true))))

(fn StopTimer
  (Variables|Default|SetIsRunning false)
  (Variables|Default|SetburntIsRunning false)
  (Variables|Default|SetTimerCompleted false)
  (Variables|Default|SetElapsedTime 0.0)
  (Development|PrintString "Reset Timer")
  (bind _returnvalue (Actor|GetActorOfClass "/Game/Blueprint/BP_TimerDisplay.BP_TimerDisplay_C"))
  (Default|SwapColor _returnvalue))

(fn UpdateTimer
  (if (Variables|Default|GetIsRunning)
    (bind _output_get (Variables|Default|SetElapsedTime (+ (Variables|Default|GetElapsedTime) 0.05)))
    (if (>= _output_get (Variables|Default|GetTimerDuration))
      (Variables|Default|SetIsRunning false)
      (Variables|Default|SetTimerCompleted true)
      (Variables|Default|SetElapsedTime 0.0)
      (Development|PrintString "Timer finished!")
      (CallFunction|SwapMesh)
      (Variables|Default|SetisCooked true)
      (CallFunction|StartTimer))))

(fn GetTimerProgress
  (return (/ (Variables|Default|GetElapsedTime) (Variables|Default|GetTimerDuration))))

(fn SwapMesh
  (params (type :type Integer))
  (bind _output_get (Variables|Default|SetTotalLocation (+ (Transformation|GetActorLocation (Utilities|Array|Get(acopy) (Variables|Default|GetActorsInside))) (Variables|Default|GetTotalLocation))))
  (if (== type 0)
    (bind _returnvalue (Game|SpawnActorfromClass "/Game/GLBs/cooked-grilledcheese/grilledCheese.grilledCheese_C" (Math|Conversions|ToTransform(Vector) _output_get) "Undefined" "MultiplyWithRoot" 0 0))
    (Variables|Default|SetcurrentFood _returnvalue)
    (else
      (Game|SpawnActorfromClass "/Game/GLBs/burnt/StaticMeshes/burnt_grilled.burnt_grilled_C" (Math|Conversions|ToTransform(Vector) _output_get) "Undefined" "MultiplyWithRoot" 0 0)))
  (Variables|Default|SetTotalLocation "0.000000,25.000000,10.000000")
  (bind (_arrayindex _arrayelement) (Utilities|Array|ReverseforEachLoop (Variables|Default|GetActorsInside))
    (:LoopBody
      (if (not (== _arrayindex 0))
        (Actor|DestroyActor _arrayelement)))))

(fn BurnUpdateTimer
  (if (Variables|Default|GetburntIsRunning)
    (bind _output_get (Variables|Default|SetElapsedTime (+ (Variables|Default|GetElapsedTime) 0.05)))
    (if (>= _output_get (Variables|Default|GetTimerDuration))
      (Variables|Default|SetburntIsRunning false)
      (Variables|Default|SetTimerCompleted true)
      (Variables|Default|SetElapsedTime 0.0)
      (Development|PrintString "Bread is BURNT")
      (Actor|DestroyActor (Variables|Default|GetcurrentFood))
      (CallFunction|SwapMesh 1))))