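; Win-condition actor that counts grilled cheeses placed in its WinZone for a VR zombie game.
; Overlap begin and end events on GrilledCheese adjust the count and refresh a BP_gcCounter display; burnt sandwiches only print a rejection.
; When the count matches the required amount, it destroys all zombie spawners and zombies and shows the win menu on the VRPawn.
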(event Custom|OnActorBeginOverlap_Event
  (params (OverlappedActor :type Actor%20Object%20Reference) (OtherActor :type Actor%20Object%20Reference))
  (bind _returnvalue (Utilities|GetClass OtherActor))
  (if (== _returnvalue "/Game/GLBs/cooked-grilledcheese/grilledCheese.grilledCheese_C")
    (bind _output_get (Variables|Default|SetGC_count (+ (Variables|Default|GetGC_count) 1)))
    (if (== (Variables|Default|GetGC_needed) _output_get)
      (Development|PrintString "YOU WINNNNNNNN" true true "(R=0.000000,G=0.660000,B=1.000000,A=1.000000)" 5.0)
      (bind _outactors (Actor|GetAllActorsOfClass "/Game/Fab/Zombie_Number_10_-_Animated/zom_10/bp_zom10_spawn.bp_zom10_spawn_C"))
      (for _array_element _outactors
        (Actor|DestroyActor _array_element))
      (bind _outactors_2 (Actor|GetAllActorsOfClass "/Game/Fab/Zombie_Number_10_-_Animated/zom_10/bp_zombie.bp_zombie_C"))
      (for _array_element_2 _outactors_2
        (Actor|DestroyActor _array_element_2))
      (bind _asvrpawn (Utilities|Casting|CastToVRPawn (Game|Player|GetPlayerPawn 0)))
      (Default|MenuVisual _asvrpawn true true)
      (else
        (bind _asbp_gc_counter (Utilities|Casting|CastToBP_gcCounter (Variables|Default|GetcounterActor)))
        (Default|SetText _asbp_gc_counter (Variables|Default|GetGC_count) (Variables|Default|GetGC_needed))))
    (elif (== _returnvalue "/Game/GLBs/burnt/StaticMeshes/burnt_grilled.burnt_grilled_C")
      (Development|PrintString "Ew. It's burnt" true true "(R=0.000000,G=0.660000,B=1.000000,A=1.000000)" 5.0))))

(event Custom|OnActorEndOverlap_Event
  (params (OverlappedActor :type Actor%20Object%20Reference) (OtherActor :type Actor%20Object%20Reference))
  (if (== (Utilities|GetClass OtherActor) "/Game/GLBs/cooked-grilledcheese/grilledCheese.grilledCheese_C")
    (Variables|Default|SetGC_count (- (Variables|Default|GetGC_count) 1))
    (bind _asbp_gc_counter (Utilities|Casting|CastToBP_gcCounter (Variables|Default|GetcounterActor)))
    (Default|SetText _asbp_gc_counter (Variables|Default|GetGC_count) (Variables|Default|GetGC_needed))))

(event EventBeginPlay
  (bind _winzone (Variables|Default|GetwinZone))
  (EventDispatchers|AssignOnActorBeginOverlap _winzone (delegate Custom|OnActorBeginOverlap_Event))
  (Collision|BindEventtoOnActorEndOverlap _winzone (delegate Custom|OnActorEndOverlap_Event))
  (bind _asbp_gc_counter (Utilities|Casting|CastToBP_gcCounter (Variables|Default|GetcounterActor)))
  (Default|SetText _asbp_gc_counter (Variables|Default|GetGC_count) (Variables|Default|GetGC_needed)))

(fn ConstructionScript)