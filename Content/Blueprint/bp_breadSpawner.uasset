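; Spawner actor that keeps buttered bread stocked at its location.
; A looping timer started on BeginPlay periodically checks the Spawn component for overlapping Bp_butteredbread actors.
; When none overlap, BreadSpawn runs a short loop that spawns new bread at the spawner's own transform.
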(event Custom|BreadSpawn
  (for _index (range 0 1)
    (Game|SpawnActorfromClass "/Game/GLBs/buttered-bread/StaticMeshes/bp_buttered-bread.bp_buttered-bread_C" (Transformation|GetActorTransform) "Undefined" "MultiplyWithRoot" 0 0)))

(event Custom|CheckForBread
  (if (== (Utilities|Array|Length (Collision|GetOverlappingActors (Variables|Default|Getspawn) "/Game/GLBs/buttered-bread/StaticMeshes/bp_buttered-bread.bp_buttered-bread_C" :!class /Script/Engine.PrimitiveComponent)) 0)
    (CallFunction|BreadSpawn)))

(event EventBeginPlay
  (Utilities|Time|SetTimerbyEvent (delegate Custom|CheckForBread) 5.0 true))

(event Collision|EventActorBeginOverlap
  (params (OtherActor :type Actor%20Object%20Reference)))

(event EventTick
  (params (DeltaSeconds :type Float%20%28single-precision%29)))

(fn ConstructionScript)