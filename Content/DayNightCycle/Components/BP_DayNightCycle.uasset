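; Day/night cycle Blueprint that rotates the directional light as the sun and counts elapsed days.
; A timeline, rate-scaled by TotalDayNightTime, drives Time and sun pitch, and the construction script sets its position to preview the chosen Time.
; A looping timer tells all BPI_IsLight actors, cached at BeginPlay, to switch on or off based on whether Time falls within night hours.
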(event Custom|CheckLight
  (for _array_element (Variables|Light|GetAllLightsInLevel)
    (Class|BPIIsLight|TurnOn/OffLight(Message) _array_element (or (Math|Float|InRange(Float) (Variables|Time|GetTime) 2e+01 24.0) (Math|Float|InRange(Float) (Variables|Time|GetTime) 0.0 6.0)))
    (Utilities|FlowControl|DoOnce false) ; enters at Reset
  ))

(event EventBeginPlay
  (bind _outactors (Actor|GetAllActorswithInterface "/Game/DayNightCycle/BlueprintInterfaces/BPI_IsLight.BPI_IsLight_C"))
  (Variables|Light|SetAllLightsInLevel _outactors)
  (Components|Timeline|SetPlayRate (Variables|Default|GetDayNightCycle_Timeline) (* (/ 1.0 (* (Variables|Time|GetTotalDayNightTime) 6e+01)) 24.0))
  (Utilities|FlowControl|Sequence
    (:then_0
      (bind (_direction _time _sun_yaw) (Timeline|DayNightCycle_Timeline Play)
        (:Update
          (Variables|Time|SetTime _time)
          (Transformation|SetWorldRotation (Variables|Default|GetDirectionalLight) (Math|Rotator|MakeRotator 0.0 _sun_yaw 0.0) false false))
        (:DayEnded
          (Math|Integer|IncrementInt (Variables|Time|GetDay)))))
    (:then_1
      (Utilities|Time|SetTimerbyEvent (delegate Custom|CheckLight) (Variables|Time|GetTotalDayNightTime) true)
      (Utilities|FlowControl|DoOnce false :!label _label
        (:Completed
          (for _array_element (Variables|Light|GetAllLightsInLevel)
            (Class|BPIIsLight|TurnOn/OffLight(Message) _array_element (or (Math|Float|InRange(Float) (Variables|Time|GetTime) 2e+01 24.0) (Math|Float|InRange(Float) (Variables|Time|GetTime) 0.0 6.0)))
            (goto _label Reset)))))))

(fn ConstructionScript
  (Components|Timeline|SetPlaybackPosition (Variables|Default|GetDayNightCycle_Timeline) (Variables|Time|GetTime) false true))