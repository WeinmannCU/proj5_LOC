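; Game state that runs the day-night cycle, tracking time of day and a day count from BeginPlay.
; A timeline starts at the stored Time at a rate derived from day length and time scale, rotating the BP_DayNightCycle directional light's pitch.
; A looping one-second timer uses an interface message to switch cached level lights on at night and off by day.
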(event Custom|CheckLight
  ;[1 1 1] Time and Day Night Cycle
  (for _array_element (Variables|Light|GetAllLightsInLevel)
    (Class|BPIIsLight|TurnOn/OffLight(Message) _array_element (or (Math|Float|InRange(Float) (Variables|Time|GetTime) 2e+01 24.0) (Math|Float|InRange(Float) (Variables|Time|GetTime) 0.0 6.0)))
    (Utilities|FlowControl|DoOnce false) ; enters at Reset
  ))

(event Custom|Start%20DayNightCycle
  ;[1 1 1] Time and Day Night Cycle
  (Utilities|FlowControl|Sequence
    (:then_0
      (bind _returnvalue (Actor|GetActorOfClass "/Game/DayNightCycle/Components/BP_DayNightCycle.BP_DayNightCycle_C"))
      (Components|Timeline|SetPlaybackPosition (Variables|Default|GetDayNightCycle_Timeline) (Variables|Time|GetTime) false true)
      (Components|Timeline|SetPlayRate (Variables|Default|GetDayNightCycle_Timeline) (/ (/ (Variables|Time|GetDayTimeInSeconds) 1.44e+03) (Variables|Time|GetTimeScale)))
      (bind (_direction _time _sunyaw) (Timeline|DayNightCycle_Timeline Play)
        (:Update
          (Variables|Time|SetTime _time)
          (Transformation|SetWorldRotation (Variables|/Game/DayNightCycle/Components/BP_DayNightCycle.BP_DayNightCycle_C|GetDirectionalLight _returnvalue) (Math|Rotator|MakeRotator 0.0 _sunyaw 0.0) false false))
        (:DayEnded
          (Math|Integer|IncrementInt (Variables|Time|GetDays)))))
    (:then_1
      (bind _outactors (Actor|GetAllActorswithInterface 0))
      (Variables|Light|SetAllLightsInLevel _outactors)
      (Utilities|Time|SetTimerbyEvent (delegate Custom|CheckLight) 1.0 true)
      (Utilities|FlowControl|DoOnce false :!label _label
        (:Completed
          (for _array_element (Variables|Light|GetAllLightsInLevel)
            (Class|BPIIsLight|TurnOn/OffLight(Message) _array_element (or (Math|Float|InRange(Float) (Variables|Time|GetTime) 2e+01 24.0) (Math|Float|InRange(Float) (Variables|Time|GetTime) 0.0 6.0)))
            (goto _label Reset)))))))

(event EventBeginPlay
  ;[1 1 1] Event BeginPlay
  (CallFunction|StartDayNightCycle))

(fn ConstructionScript)